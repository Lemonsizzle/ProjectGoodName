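; Locked gate actor that opens when the player enters its trigger box while carrying at least one key.
; Overlap unlocks it, consumes a key from BP_FirstPersonCharacter and disables collision on the whole actor.
; The OpenUp_down timeline then lowers the Door by lerping toward an offset below its current relative location, re-read each update, so movement accumulates.
; Nothing relocks or closes it.
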(event `self.Box.OnComponentBeginOverlap`
  (params (OverlappedComponent :type "PrimitiveComponent Object Reference") (OtherActor :type "Actor Object Reference") (OtherComp :type "PrimitiveComponent Object Reference") (OtherBodyIndex :type Integer) (bFromSweep :type Boolean) (SweepResult :type "HitResult Structure (by ref)"))
  (bind _returnvalue (`GameplayStatics.GetPlayerCharacter` 0))
  (bind _relativelocation (`SceneComponent.RelativeLocation` (`self.door`)))
  (bind _asbp_first_person_character (cast `/Game/FirstPerson/Blueprints/BP_FirstPersonCharacter` _returnvalue))
  (bind _keys (`/Game/FirstPerson/Blueprints/BP_FirstPersonCharacter.Keys` _asbp_first_person_character))
  (if (and (== OtherActor _returnvalue) (> _keys 0) (`self.Locked`))
    (`self.SetActorEnableCollision` false)
    (set `self.Locked` false)
    (`/Engine/EditorBlueprintResources/StandardMacros.DecrementInt` _keys
      (:`  `
        (bind (_direction _open) (`Timeline|open up_down`)
          (:`Update`
            (`SceneComponent.K2_SetRelativeLocation` (`self.door`) (`KismetMathLibrary.VLerp` _relativelocation (- _relativelocation (0.0 0.0 100.0)) _open) false false)))))))

(fn `UserConstructionScript`)