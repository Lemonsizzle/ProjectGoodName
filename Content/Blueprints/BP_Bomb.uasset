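; BP_Bomb is an explosive actor that fractures and scatters Chaos destructibles when its Explode event is called.
; Explode spawns the explosion particles and sound, applies two physics fields, then destroys the actor.
; An external cluster strain field sized by the Sphere component breaks clusters.
; A radial linear velocity field, culled outside that same sphere via a culling field, pushes pieces outward from its center.
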(event `Explode`
  (bind _returnvalue (`self.K2_GetActorLocation`))
  (bind _fieldsystem (`self.FieldSystem`))
  (bind _sphere (`self.Sphere`))
  (bind _returnvalue_2 (`SceneComponent.K2_GetComponentLocation` _sphere))
  (bind _returnvalue_3 (`RadialFalloff.SetRadialFalloff` (`self.RadialFalloff`) 500000.0 0.0 1.0 0.0 (`SphereComponent.GetScaledSphereRadius` _sphere) _returnvalue_2 "Field_FallOff_None"))
  (`GameplayStatics.SpawnEmitterAtLocation` "/Game/StarterContent/Particles/P_Explosion.P_Explosion" _returnvalue)
  (`GameplayStatics.PlaySoundAtLocation` "/Game/StarterContent/Audio/Explosion_Cue.Explosion_Cue" _returnvalue (struct) 1.0 1.0 0.0 null null null null)
  (`FieldSystemComponent.ApplyPhysicsField` _fieldsystem true "Field_ExternalClusterStrain" null _returnvalue_3)
  (`FieldSystemComponent.ApplyPhysicsField` _fieldsystem true "Field_LinearVelocity" null (`CullingField.SetCullingField` (`self.CullingField`) _returnvalue_3 (`RadialVector.SetRadialVector` (`self.RadialVector`) 1000.0 _returnvalue_2) "Field_Culling_Outside"))
  (`self.K2_DestroyActor`))

(fn `UserConstructionScript`)