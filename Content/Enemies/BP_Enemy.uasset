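; BP_Enemy is an enemy character with health, death handling and an adjustable walk speed.
; Damage lowers Health, and at zero or below the enemy is unpossessed from its controller and loses capsule collision.
; The Unpossessed event carries out the death: it sets Dead, ragdolls the mesh and destroys the actor after a short delay.
; A helper function sets the movement component's max walk speed.
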(event `/Game/Interfaces/BPI_Damageable.TakeDamage`
  (params (Damage :type Integer))
  (bind _output_get (set `self.Health` (- (`self.Health`) Damage)))
  (if (<= _output_get 0)
    (if (not (`self.Dead`))
      (`Controller.UnPossess` (`self.GetController`))
      (`PrimitiveComponent.SetCollisionEnabled` (`self.CapsuleComponent`) "NoCollision"))))

(event `self.ReceiveUnpossessed`
  (params (OldController :type "Controller Object Reference"))
  (set `self.Dead` true)
  (`PrimitiveComponent.SetSimulatePhysics` (`self.Mesh`) true)
  (`KismetSystemLibrary.Delay` 5.0)
  (`self.K2_DestroyActor`))

(fn `Update Walk Speed`
  (params (`New Walk Speed` :type "Float (double-precision)"))
  (set `CharacterMovementComponent.MaxWalkSpeed` `New Walk Speed` (`self.CharacterMovement`)))

(fn `UserConstructionScript`)